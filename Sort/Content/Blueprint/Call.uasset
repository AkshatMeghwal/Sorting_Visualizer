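; Input-handling actor that enables player input on BeginPlay and triggers sort start, fast-forward and spawning.
; StartSort clears a nonzero Flag, records Time into Sttime and prints a debug message.
; Holding TimeSpeed raises global time dilation until released, and Spawn calls Spawningproc.
; Sorting and spawning logic are not defined in these graphs.
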(event EventBeginPlay
  (Input|EnableInput (Game|GetPlayerController 0)))

(event Collision|EventActorBeginOverlap
  (params (OtherActor :type Actor%20Object%20Reference)))

(event EventTick
  (params (DeltaSeconds :type Float%20%28single-precision%29)))

(event Input|ActionEvents|InputActionStartSort
  (params (Key :type Key%20Structure :default "None"))
  ;[1 1 1] Flag Changing jutsu..
  (:Pressed
    (if (Math|Conversions|ToBoolean(Integer) (Variables|Default|Getflag))
      (Variables|Default|Setflag 0)
      (Variables|Default|Setsttime (Variables|Default|Gettime))
      (Development|PrintString "F is pressed " true true "(R=0.000000,G=0.660000,B=1.000000,A=1.000000)" 1e+01 "1"))))

(event Input|ActionEvents|InputActionTimeSpeed
  (params (Key :type Key%20Structure :default "None"))
  (:Pressed
    (Utilities|Time|SetGlobalTimeDilation 1e+01))
  (:Released
    (Utilities|Time|SetGlobalTimeDilation 1.0)))

(event Input|ActionEvents|InputActionSpawn
  (params (Key :type Key%20Structure :default "None"))
  (:Pressed
    (Class|MyActor|Spawningproc)))

(fn ConstructionScript)